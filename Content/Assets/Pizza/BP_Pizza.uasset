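; BP_Pizza is a pizza that can change appearance to look cooked or boxed.
; On BeginPlay it creates a dynamic material instance from MI_Pizza and applies it to its mesh.
; SetCookedMaterial sets that instance's BakedColor parameter to grey to show baking.
; SetBoxedMesh swaps in the boxed static mesh, rescales it and replaces the dynamic material with the box material.
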(event EventBeginPlay
  (bind _mesh (Variables|Character|GetMesh))
  (bind _returnvalue (Rendering|Material|CreateDynamicMaterialInstance _mesh 0 "/Game/Assets/Pizza/Models/Materials/MI_Pizza.MI_Pizza" "None" :!class /Script/Engine.PrimitiveComponent))
  (bind _output_get (Variables|Default|SetDynamicMaterial _returnvalue))
  (Rendering|Material|SetMaterial _mesh 0 _output_get))

(event EventSetCookedMaterial
  (Rendering|Material|SetVectorParameterValue (Variables|Default|GetDynamicMaterial) "BakedColor" "(R=0.400000,G=0.400000,B=0.400000,A=1.000000)" :!class /Script/Engine.MaterialInstanceDynamic))

(event EventSetBoxedMesh
  (bind _mesh (Variables|Character|GetMesh))
  (Components|StaticMesh|SetStaticMesh _mesh (Variables|Default|GetBoxedMesh))
  (Transformation|SetWorldScale3D _mesh "3.000000,3.000000,3.000000")
  (Rendering|Material|SetMaterial _mesh 0 "/Game/Assets/Pizza/Models/Materials/M_Box002Mat.M_Box002Mat"))

(fn ConstructionScript)